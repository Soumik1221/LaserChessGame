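; BP_BoardPawn is a laser chess board piece whose appearance follows its pawn type and team.
; A type change event swaps the static mesh among Laser, King, Switch, Defender and Deflector models.
; A team change event calls a helper that finds the team and body material slots by name and tints dynamic material instances, red or blue for team, dark or light for body.
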(event EventBeginPlay)

(event Collision|EventActorBeginOverlap
  (params (OtherActor :type Actor%20Object%20Reference)))

(event EventTick
  (params (DeltaSeconds :type Float%20%28single-precision%29)))

(event EventOnPawnTypeChanged
  (params (OutType :type EPawnType%20Enum :default "EPT_Laser"))
  ;[1 1 1] Set Pawn Mesh
  (Components|StaticMesh|SetStaticMesh (Variables|Default|GetPawnMesh) (Utilities|Select :Index OutType :EPT_Laser "/Game/Mesh/Dev_LaserChess_Laser.Dev_LaserChess_Laser" :EPT_King "/Game/Mesh/Dev_LaserChess_King.Dev_LaserChess_King" :EPT_Switch "/Game/Mesh/Dev_LaserChess_Switch.Dev_LaserChess_Switch" :EPT_Defender "/Game/Mesh/Dev_LaserChess_Defender.Dev_LaserChess_Defender" :EPT_Deflector "/Game/Mesh/Dev_LaserChess_Deflector.Dev_LaserChess_Deflector")))

(event EventOnPawnTeamChanged
  (params (OutTeam :type EPawnTeam%20Enum :default "EPT_TeamA"))
  ;[1 1 1] Set Color
  (CallFunction|HelperSetMaterialColor "Mat_Team" OutTeam "(R=1.000000,G=0.000000,B=0.000000,A=1.000000)" "(R=0.000000,G=0.000000,B=1.000000,A=1.000000)")
  (CallFunction|HelperSetMaterialColor "Mat_Body" OutTeam "(R=0.151042,G=0.151042,B=0.151042,A=1.000000)" "(R=0.879623,G=0.879623,B=0.879623,A=1.000000)"))

(fn ConstructionScript)

(fn HelperSetMaterialColor
  (params (Slot%20Name :type Name) (Team :type EPawnTeam%20Enum :default "EPT_TeamA") (Team%20A%20Color :type Linear%20Color%20Structure) (Team%20B%20Color :type Linear%20Color%20Structure))
  (bind _pawnmesh (Variables|Default|GetPawnMesh))
  (bind _returnvalue (Class|MeshComponent|GetMaterialSlotNames _pawnmesh))
  (bind _returnvalue_2 (Utilities|Array|FindItem _returnvalue Slot%20Name))
  (if (>= _returnvalue_2 0)
    (bind _returnvalue_3 (Rendering|Material|CreateDynamicMaterialInstance _pawnmesh _returnvalue_2 0 "Team_Material" :!class /Script/Engine.PrimitiveComponent))
    (LocalVariables|SetLocal_MatInst _returnvalue_3)
    (bind _local_matinst (LocalVariables|GetLocal_MatInst)
      (:then
        (Rendering|Material|SetVectorParameterValue _local_matinst "Base Color" (Math|Color|SelectColor Team%20A%20Color Team%20B%20Color (Utilities|Enum|Equal(Enum) Team "EPT_TeamA")) :!class /Script/Engine.MaterialInstanceDynamic))
      (:else))))